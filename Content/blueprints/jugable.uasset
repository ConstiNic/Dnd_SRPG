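; Playable pawn Blueprint ("jugable") with axis-driven movement and a mouse-wheel camera zoom.
; MoveForward and MoveRight add movement input along the control rotation's forward and right vectors.
; Wheel up plays one timeline forward and wheel down reverses another, gated by CineCamera relative Z and X respectively.
; The SetRelativeLocation nodes reading those timeline tracks never execute, so the zoom does not move the camera.
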(event Input|AxisEvents|InputAxisMoveForward
  (params (AxisValue :type Float%20%28single-precision%29))
  ;[1 1 1] movimiento
  (Pawn|Input|AddMovementInput (Math|Vector|GetForwardVector (Pawn|GetControlRotation :!class /Script/Engine.Pawn)) AxisValue false))

(event Input|AxisEvents|InputAxisMoveRight
  (params (AxisValue :type Float%20%28single-precision%29))
  ;[1 1 1] movimiento
  (Pawn|Input|AddMovementInput (Math|Vector|GetRightVector (Pawn|GetControlRotation :!class /Script/Engine.Pawn)) AxisValue false))

(event Input|MouseEvents|MouseWheelUp
  (params (Key :type Key%20Structure :default "None"))
  ;[1 1 1] zoom de la camara
  (:Pressed
    (if (>= (.z (Variables|/Script/Engine.SceneComponent|GetRelativeLocation (Variables|Default|GetCineCamera))) 7.3e+02)
      (bind _newtrack_0 (Timeline|Línea%20de%20tiempo_0 PlayFromStart)))))

(event Input|MouseEvents|MouseWheelDown
  (params (Key :type Key%20Structure :default "None"))
  ;[1 1 1] zoom de la camara
  (:Pressed
    (if (>= (.x (Variables|/Script/Engine.SceneComponent|GetRelativeLocation (Variables|Default|GetCineCamera))) 170.263321)
      (bind _newtrack_0 (Timeline|Línea%20de%20tiempo_1 ReverseFromEnd)))))

(fn ConstructionScript)